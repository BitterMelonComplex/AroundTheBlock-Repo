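; Garlic NPC that wanders the navmesh and reacts with a flee when it sees a pawn.
; RandomRoam moves to random nearby points, re-rolling after a pause or when a forward line trace hits something.
; PawnSensing triggers a hop montage whose notify shows a surprise marker and squeak, then a faster AI move before roaming resumes.
; ContinueDialogue updates the player's boost, notifies the garlic spawner and destroys the actor.
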(event OnSeePawn(PawnSensing)
  (params (Pawn :type Pawn%20Object%20Reference))
  (CallFunction|Flee Pawn))

(event Custom|Random%20Roam
  ;[1 1 1] Random Roam Logic
  (Variables|/Script/Engine.CharacterMovementComponent|SetMaxWalkSpeed (Variables|Character|GetCharacterMovement) (Variables|Default|GetNormal%20Walk%20Speed))
  (bind _randomlocation (Class|NavigationSystemV1|GetRandomLocationinNavigableRadius (Transformation|GetActorLocation) 1e+03 0 0))
  (AI|AIMoveTo self _randomlocation 0 5.0 false
    (:OnSuccess
      (Utilities|FlowControl|Delay 5.0)
      (CallFunction|RandomRoam))))

(event Custom|Flee
  (params (pawn :type Pawn%20Object%20Reference))
  (bind _returnvalue (Transformation|GetActorLocation))
  (bind _surprise_marker (Variables|Default|Getsurprise%20marker))
  ;[1 1 1] Fleeing Logic
  (if (not (Variables|Default|GetIsFleeing))
    (Animation|Montage|PlayMontage (Variables|Character|GetMesh) "/Game/Characters/Garlic/Garlic_Hop_Montage.Garlic_Hop_Montage" 2.0 0.0 ""
      (:then
        (Utilities|FlowControl|Delay 0.5)
        (Variables|/Script/Engine.CharacterMovementComponent|SetMaxWalkSpeed (Variables|Character|GetCharacterMovement) (Variables|Default|GetFlee%20Walk%20Speed))
        (AI|AIMoveTo (AI|GetAIController self) (+ _returnvalue (* (Math|Vector|GetForwardVector (Math|Rotator|FindLookatRotation _returnvalue (Transformation|GetActorLocation pawn))) (Variables|Default|GetFlee%20Distance))) 0 -1.0 "Default" "Default" true false
          (:OnRequestFailed
            _)
          (:OnMoveFinished
            _))
        (Variables|Default|SetIsFleeing false)
        (Variables|/Script/Engine.CharacterMovementComponent|SetMaxWalkSpeed (Variables|Character|GetCharacterMovement) (Variables|Default|GetNormal%20Walk%20Speed))
        (Utilities|FlowControl|Delay 0.5)
        (CallFunction|RandomRoam))
      (:OnNotifyBegin
        (Utilities|FlowControl|DoOnce false :!label _label
          (:Completed
            ;;[1 0 0] Surprised marker and Squeak Audio
            (Rendering|SetVisibility _surprise_marker true false)
            (Audio|Components|Audio|Play (Variables|Default|GetSqueak) 0.0)
            (Utilities|FlowControl|Delay 2.0)
            (Rendering|SetVisibility _surprise_marker false false)
            (Audio|Components|Audio|Stop (Variables|Default|GetSqueak))
            (goto _label Reset)))))))

(event EventBeginPlay
  (bind _asbp_third_person_character (Utilities|Casting|CastToBP_ThirdPersonCharacter (Game|GetPlayerCharacter 0)))
  (Variables|Default|SetPlayer%20Ref _asbp_third_person_character)
  (Rendering|SetVisibility (Variables|Default|Getsurprise%20marker) false false)
  (CallFunction|RandomRoam))

(event EventTick
  (params (DeltaSeconds :type Float%20%28single-precision%29))
  (bind _returnvalue (Transformation|GetActorLocation))
  ;[1 1 1] Fleeing Logic
  ;;[0.09356 0.6762 1] Dectect if hit anything
  (bind _returnvalue_2 (Collision|LineTraceByChannel _returnvalue (+ _returnvalue (* (Math|Rotator|GetRotationXVector (Transformation|GetActorRotation)) 1e+02)) "TraceTypeQuery1" false 0 "None"))
  (if _returnvalue_2
    (CallFunction|RandomRoam)))

(event EventContinueDialogue
  (Default|UpdateBoostValue (Variables|Default|GetPlayer%20Ref) 1.0)
  (Default|OnGarlicDestroyed (Variables|Default|GetGarlic%20Spawner))
  (Actor|DestroyActor))

(fn ConstructionScript)