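; BP_Beetle is an NPC beetle character with blinking eyes that can be startled into fleeing.
; Flee plays a stunned effect and dazed montage, then a launched jump whose montage notify flashes a surprise marker and squeak.
; It then raises walk speed to the flee value and uses AI MoveTo toward the nearest BP_Beetle_DestroyBox.
; ContinueDialogue notifies the BeetleSpawner and destroys the beetle, while blinking runs as a self-calling material-swap loop.
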(event Custom|Blinking
  (bind _mesh (Variables|Character|GetMesh))
  ;[1 1 1] Blinking
  (Rendering|Material|SetMaterial _mesh 1 "/Game/Characters/Beetle/M_BeetleEye1.M_BeetleEye1")
  (Utilities|FlowControl|Delay 0.2)
  (Rendering|Material|SetMaterial _mesh 1 "/Game/Characters/Beetle/M_BeetleEye2.M_BeetleEye2")
  (Utilities|FlowControl|Delay 0.2)
  (CallFunction|Blinking))

(event Custom|Flee
  ;[1 1 1] Flee to destroy box Logic
  (Variables|Default|SetShortest%20%20Distance 9999999.0)
  (if (not (Variables|Default|GetIsFleeing))
    (Utilities|FlowControl|DoOnce false :!label _label
      (:Completed
        (Niagara|SpawnSystemAttached "/Game/FX/NS_Stunned_Beetle.NS_Stunned_Beetle" (Variables|Default|GetStunned%20FX%20Area) "" (Math|Vector|MakeVector 0.0 0.0 0.0) "0, 0, 0" "KeepRelativeOffset" true)
        (Animation|PlayAnimMontage "/Game/Characters/Beetle/Beetle_Dazed_Montage.Beetle_Dazed_Montage" 1.0 "None")
        (Utilities|FlowControl|Delay 1.3)
        (Character|LaunchCharacter "0.000000,0.000000,300.000000" false false)
        (Animation|Montage|PlayMontage (Variables|Character|GetMesh) "/Game/Characters/Beetle/Beetle_Jump_Montage.Beetle_Jump_Montage"
          (:then
            (Utilities|FlowControl|Delay 0.2)
            ;;[0.2576 1 0.3813] Find closest destroy box and run to it
            (bind _outactors (Actor|GetAllActorsOfClass "/Game/Blueprints/BP_Beetle_DestroyBox.BP_Beetle_DestroyBox_C"))
            (Utilities|IsValid (.ReturnValue (Actor|FindNearestActor (Transformation|GetActorLocation) _outactors))
              (:Is%20Valid
                (if (< (.Distance (Actor|FindNearestActor (Transformation|GetActorLocation) _outactors)) (Variables|Default|GetShortest%20%20Distance))
                  (Variables|Default|SetShortest%20%20Distance 0.0)
                  ;;;[1 1 1] Set movement speed
                  (Variables|/Script/Engine.CharacterMovementComponent|SetMaxWalkSpeed (Variables|Character|GetCharacterMovement) (Variables|Default|GetFlee%20Walk%20Speed))
                  (AI|AIMoveTo self "0, 0, 0" (.ReturnValue (Actor|FindNearestActor (Transformation|GetActorLocation) _outactors)) 5.0 false
                    (:then
                      (goto _label Reset)))))))
          (:OnNotifyBegin
            ;;[1 0.7256 0.003805] Show surprise marker
            (Rendering|SetVisibility (Variables|Default|GetSurprise%20Marker) true false)
            (Audio|Components|Audio|Play (Variables|Default|GetSqueak) 0.0)
            (Utilities|FlowControl|Delay 0.8)
            (Rendering|SetVisibility (Variables|Default|GetSurprise%20Marker) false false)
            (Audio|Components|Audio|Stop (Variables|Default|GetSqueak))))))))

(event EventBeginPlay
  (Utilities|FlowControl|Sequence
    (:then_0
      (CallFunction|Blinking))
    (:then_1
      (Rendering|SetVisibility (Variables|Default|GetSurprise%20Marker) false false))
    (:then_2
      (Rendering|Material|SetMaterial (Variables|Character|GetMesh) 0 (Variables|Default|GetBeetle%20Material)))))

(event EventContinueDialogue
  ;[1 1 1] Destroy beetle
  (Default|OnBeetleDestroyed (Variables|Default|GetBeetle%20Spawner))
  (Actor|DestroyActor))

(fn ConstructionScript)