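; BP_Vern is a quest NPC that faces the player every tick and plays spawn and despawn animations on player events.
; Overlapping its dialogue collision shows data-table dialogue on the player's HUD; wearing the required hat also advances dialogue and sets the quest once.
; ContinueDialogue steps through linked rows, clearing the matching quest at the terminal row.
; OnFinished adds the quest row's hat and stamp rewards to the player's inventory.
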(event OnComponentBeginOverlap(DialogueCollision)
  (params (OverlappedComponent :type Primitive%20Component%20Object%20Reference) (OtherActor :type Actor%20Object%20Reference) (OtherComp :type Primitive%20Component%20Object%20Reference) (OtherBodyIndex :type Integer) (bFromSweep :type Boolean) (SweepResult :type Hit%20Result%20Structure%20%28by%20ref%29))
  (bind _player_ref (Variables|Default|GetPlayer%20Ref))
  (bind _vern_dialogue_component (Variables|Default|GetVern%20Dialogue%20Component))
  (bind _playerhud (Variables|/Game/Player_Blueprints/BP_ThirdPersonCharacter.BP_ThirdPersonCharacter_C|GetPlayerHUD _player_ref))
  (if (== OtherActor _player_ref)
    (if (== (Variables|/Game/Player_Blueprints/BP_ThirdPersonCharacter.BP_ThirdPersonCharacter_C|GetEquippedHatID _player_ref) (Variables|Default|GetRequiredHatID))
      (Utilities|FlowControl|DoOnce false
        (:Completed
          (Default|ProgressDialogue (Variables|Default|GetVern%20Dialogue%20Component))
          (Default|UpdateCurrentQuest (Variables|Default|GetPlayer%20Ref) (.rowname (Variables|Default|GetQuestInfo))))))
    (Default|ActivateDialogueWidget _playerhud)
    (bind _returnvalue (Utilities|GetDataTableRow (Variables|/Game/Blueprints/AC_Dialogue.AC_Dialogue_C|GetDialogueDataTable _vern_dialogue_component) (Variables|/Game/Blueprints/AC_Dialogue.AC_Dialogue_C|GetStartingDialogueRow _vern_dialogue_component))
      (:then
        (Default|UpdateDialogueText _playerhud (.DialogueText (Utilities|Struct|BreakS_Dialogue _returnvalue)))
        (Variables|Default|SetNext%20Row (.NextRow (Utilities|Struct|BreakS_Dialogue _returnvalue)))))))

(event OnComponentEndOverlap(DialogueCollision)
  (params (OverlappedComponent :type Primitive%20Component%20Object%20Reference) (OtherActor :type Actor%20Object%20Reference) (OtherComp :type Primitive%20Component%20Object%20Reference) (OtherBodyIndex :type Integer))
  (bind _player_ref (Variables|Default|GetPlayer%20Ref))
  (if (== OtherActor _player_ref)
    (Default|DeactivateDialogueWidget (Variables|/Game/Player_Blueprints/BP_ThirdPersonCharacter.BP_ThirdPersonCharacter_C|GetPlayerHUD _player_ref))))

(event Custom|Play%20DeSpawn%20Montage
  (Components|Animation|PlayAnimation (Variables|Character|GetMesh) "/Game/Characters/Vern/Animations/Vern_DeSpawn.Vern_DeSpawn" false))

(event Custom|Play%20Spawn%20Montage
  (bind _mesh (Variables|Character|GetMesh))
  ;[1 1 1] Spawn animations
  (Components|Animation|PlayAnimation _mesh "/Game/Characters/Vern/Animations/Vern_Jump.Vern_Jump" false)
  (Utilities|FlowControl|Delay 1.62)
  (Components|Animation|PlayAnimation _mesh "/Game/Characters/Vern/Animations/Vern_Idle.Vern_Idle" true))

(event EventBeginPlay
  (bind _asbp_third_person_character (Utilities|Casting|CastToBP_ThirdPersonCharacter (Game|GetPlayerCharacter 0)))
  (bind _output_get (Variables|Default|SetPlayer%20Ref _asbp_third_person_character))
  (EventDispatchers|BindEventtoOnVernSpawn _output_get (delegate Custom|Play%20Spawn%20Montage))
  (EventDispatchers|BindEventtoOnVernDeSpawn _output_get (delegate Custom|Play%20DeSpawn%20Montage)))

(event EventContinueDialogue
  (bind _player_ref (Variables|Default|GetPlayer%20Ref))
  (bind _playerhud (Variables|/Game/Player_Blueprints/BP_ThirdPersonCharacter.BP_ThirdPersonCharacter_C|GetPlayerHUD _player_ref))
  (bind _returnvalue (Utilities|GetDataTableRow (Variables|/Game/Blueprints/AC_Dialogue.AC_Dialogue_C|GetDialogueDataTable (Variables|Default|GetVern%20Dialogue%20Component)) (Variables|Default|GetNext%20Row))
    (:then
      (Default|UpdateDialogueText _playerhud (.DialogueText (Utilities|Struct|BreakS_Dialogue _returnvalue)))
      (bind _output_get (Variables|Default|SetNext%20Row (.NextRow (Utilities|Struct|BreakS_Dialogue _returnvalue))))
      (if (== _output_get "0")
        (bind _currentquest (Default|GetCurrentQuest (Variables|Default|GetPlayer%20Ref)))
        (if (== _currentquest (.rowname (Variables|Default|GetQuestInfo)))
          (Default|UpdateCurrentQuest (Variables|Default|GetPlayer%20Ref) "None"))))
    (:RowNotFound
      (Default|DeactivateDialogueWidget _playerhud))))

(event EventTick
  (params (DeltaSeconds :type Float%20%28single-precision%29))
  ;[1 1 1] Look at player
  (Transformation|SetActorRotation (Math|Rotator|FindLookatRotation (Transformation|GetActorLocation) (Transformation|GetActorLocation (Game|GetPlayerCharacter 0)))))

(event EventOnFinished
  (bind _player_ref (Variables|Default|GetPlayer%20Ref))
  (bind _questinfo (Variables|Default|GetQuestInfo))
  (bind _inventorycomponent (Variables|/Game/Player_Blueprints/BP_ThirdPersonCharacter.BP_ThirdPersonCharacter_C|GetInventoryComponent _player_ref))
  (bind _returnvalue (Utilities|GetDataTableRow (.datatable _questinfo) (.rowname _questinfo))
    (:then
      (Default|AddtoInventory _inventorycomponent (.RewardsHatWithID (Utilities|Struct|BreakS_QuestInfo _returnvalue)))
      (Default|AddtoInventory _inventorycomponent (.RewardsStampWithID (Utilities|Struct|BreakS_QuestInfo _returnvalue))))))

(fn ConstructionScript)