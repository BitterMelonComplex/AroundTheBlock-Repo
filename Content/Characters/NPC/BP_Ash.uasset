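; BP_Ash is the Blueprint for the Ash NPC, giving the character a looping eye blink.
; On BeginPlay it starts the blink and caches the third-person player character in PlayerRef, which this graph does not otherwise use.
; The Blinking event swaps one mesh material slot through closed, half-open and open eye materials using Delays, then calls itself to repeat indefinitely.
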(event Custom|Blinking
  (bind _mesh (Variables|Character|GetMesh))
  ;[1 1 1] Blinking sequence
  (Rendering|Material|SetMaterial _mesh 8 "/Game/Characters/Ash/Ash_eye_closed.Ash_eye_closed")
  (Utilities|FlowControl|Delay 0.2)
  (Rendering|Material|SetMaterial _mesh 8 "/Game/Characters/Ash/Ash_eye_halfopen.Ash_eye_halfopen")
  (Utilities|FlowControl|Delay 0.1)
  (Rendering|Material|SetMaterial _mesh 8 "/Game/Characters/Ash/Ash_eye_open.Ash_eye_open")
  (Utilities|FlowControl|Delay 4.0)
  (CallFunction|Blinking))

(event EventBeginPlay
  (CallFunction|Blinking)
  (bind _asbp_third_person_character (Utilities|Casting|CastToBP_ThirdPersonCharacter (Game|GetPlayerCharacter 0)))
  (Variables|Default|SetPlayer%20Ref _asbp_third_person_character))

(event Collision|EventActorBeginOverlap
  (params (OtherActor :type Actor%20Object%20Reference)))

(event EventTick
  (params (DeltaSeconds :type Float%20%28single-precision%29)))

(fn ConstructionScript)