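; BP_Vern is the Vern character, which animates its spawn and despawn and keeps facing the player.
; On BeginPlay it binds to the OnVernSpawn and OnVernDeSpawn events on BP_ThirdPersonCharacter.
; Spawning plays a jump animation, then switches to a looping idle after a fixed delay, while despawning plays a one-shot animation.
; Tick sets the full actor rotation toward the player's location every frame.
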(event Custom|Play%20DeSpawn%20Montage
  (Components|Animation|PlayAnimation (Variables|Character|GetMesh) "/Game/Characters/Vern/Animations/Vern_DeSpawn.Vern_DeSpawn" false))

(event Custom|Play%20Spawn%20Montage
  (bind _mesh (Variables|Character|GetMesh))
  ;[1 1 1] Spawn animations
  (Components|Animation|PlayAnimation _mesh "/Game/Characters/Vern/Animations/Vern_Jump.Vern_Jump" false)
  (Utilities|FlowControl|Delay 1.62)
  (Components|Animation|PlayAnimation _mesh "/Game/Characters/Vern/Animations/Vern_Idle.Vern_Idle" true))

(event EventBeginPlay
  (bind _asbp_third_person_character (Utilities|Casting|CastToBP_ThirdPersonCharacter (Game|GetPlayerCharacter 0)))
  (bind _output_get (Variables|Default|SetPlayer%20Ref _asbp_third_person_character))
  (EventDispatchers|BindEventtoOnVernSpawn _output_get (delegate Custom|Play%20Spawn%20Montage))
  (EventDispatchers|BindEventtoOnVernDeSpawn _output_get (delegate Custom|Play%20DeSpawn%20Montage)))

(event EventTick
  (params (DeltaSeconds :type Float%20%28single-precision%29))
  ;[1 1 1] Look at player
  (Transformation|SetActorRotation (Math|Rotator|FindLookatRotation (Transformation|GetActorLocation) (Transformation|GetActorLocation (Game|GetPlayerCharacter 0)))))

(fn ConstructionScript)