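; Flower pickup-style actor that plays a sniff sound and summons Vern while the player is within its spawn radius.
; Construction sets the flower mesh and item info from a data table row.
; Entering the radius spawns BP_Vern at the flower with a required hat ID and notifies the player character.
; Leaving stops the sound, notifies the player, then destroys all Vern actors after delays; TriggerZone overlaps have no effect.
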(event OnComponentBeginOverlap(TriggerZone)
  (params (OverlappedComponent :type Primitive%20Component%20Object%20Reference) (OtherActor :type Actor%20Object%20Reference) (OtherComp :type Primitive%20Component%20Object%20Reference) (OtherBodyIndex :type Integer) (bFromSweep :type Boolean) (SweepResult :type Hit%20Result%20Structure%20%28by%20ref%29))
  (bind _asbp_third_person_character (Utilities|Casting|CastToBP_ThirdPersonCharacter OtherActor))
  (Utilities|IsValid _asbp_third_person_character))

(event OnComponentEndOverlap(TriggerZone)
  (params (OverlappedComponent :type Primitive%20Component%20Object%20Reference) (OtherActor :type Actor%20Object%20Reference) (OtherComp :type Primitive%20Component%20Object%20Reference) (OtherBodyIndex :type Integer))
  (bind _asbp_third_person_character (Utilities|Casting|CastToBP_ThirdPersonCharacter OtherActor))
  (Utilities|IsValid _asbp_third_person_character))

(event OnComponentBeginOverlap(VernSpawnRadius)
  (params (OverlappedComponent :type Primitive%20Component%20Object%20Reference) (OtherActor :type Actor%20Object%20Reference) (OtherComp :type Primitive%20Component%20Object%20Reference) (OtherBodyIndex :type Integer) (bFromSweep :type Boolean) (SweepResult :type Hit%20Result%20Structure%20%28by%20ref%29))
  ;[1 1 1] Spawns and De-Spawns Vern
  (bind _asbp_third_person_character (Utilities|Casting|CastToBP_ThirdPersonCharacter OtherActor))
  (Utilities|IsValid _asbp_third_person_character
    (:Is%20Valid
      ;;[0.08137 1 0] Play Audio
      (Variables|Default|SetIsOverlapping? true)
      (Audio|Components|Audio|Play (Variables|Default|GetSniff) 0.0)
      (Development|PrintString "Sniff Sniff")
      (Development|PrintString "Vern will spawn")
      (if (not (Variables|Default|GetIs%20Vern%20Spawned?))
        (Utilities|FlowControl|Delay 0.2)
        (bind _returnvalue (Game|SpawnActorfromClass "/Game/Characters/NPC/BP_Vern.BP_Vern_C" (Math|Transform|MakeTransform (Transformation|GetWorldLocation (Variables|Default|GetFlower)) "0, 0, 0" "1.000000,1.000000,1.000000") "Undefined" "MultiplyWithRoot" 0 (Variables|Default|GetVernHatIDCheck) 0))
        (Utilities|IsValid _returnvalue
          (:Is%20Valid
            (Default|CallOnVernSpawn (Variables|Default|GetPlayer%20Ref))
            (Variables|Default|SetIs%20Vern%20Spawned? true)))))))

(event OnComponentEndOverlap(VernSpawnRadius)
  (params (OverlappedComponent :type Primitive%20Component%20Object%20Reference) (OtherActor :type Actor%20Object%20Reference) (OtherComp :type Primitive%20Component%20Object%20Reference) (OtherBodyIndex :type Integer))
  ;[1 1 1] Spawns and De-Spawns Vern
  (bind _asbp_third_person_character (Utilities|Casting|CastToBP_ThirdPersonCharacter OtherActor))
  (Utilities|IsValid _asbp_third_person_character
    (:Is%20Valid
      ;;[0 1 0.2335] Stop Audio
      (Variables|Default|SetIsOverlapping? false)
      (Audio|Components|Audio|Stop (Variables|Default|GetSniff))
      (Development|PrintString "Vern will leave")
      (if (Variables|Default|GetIs%20Vern%20Spawned?)
        (Utilities|FlowControl|Delay 1.0)
        (Default|CallOnVernDeSpawn (Variables|Default|GetPlayer%20Ref))
        (Utilities|FlowControl|Delay 1.62)
        (bind _outactors (Actor|GetAllActorsOfClass "/Game/Characters/NPC/BP_Vern.BP_Vern_C"))
        (Actor|DestroyActor _outactors)
        (Variables|Default|SetIs%20Vern%20Spawned? false)))))

(event EventBeginPlay
  (bind _asbp_third_person_character (Utilities|Casting|CastToBP_ThirdPersonCharacter (Game|GetPlayerCharacter 0)))
  (Variables|Default|SetPlayer%20Ref _asbp_third_person_character))

(fn ConstructionScript
  (bind _item (Variables|Default|GetItem))
  (bind _returnvalue (Utilities|GetDataTableRow (.datatable _item) (.rowname _item))
    (:then
      (Components|StaticMesh|SetStaticMesh (Variables|Default|GetFlower) (.ItemMesh1 (Utilities|Struct|BreakS_Flower _returnvalue)))
      (Variables|Default|SetItem%20Info _returnvalue))))