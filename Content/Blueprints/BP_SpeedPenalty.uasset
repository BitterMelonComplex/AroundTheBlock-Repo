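; BP_SpeedPenalty is a trigger zone that caps the third-person character's sprint speed while the character is inside it.
; TriggerBox overlap events cast the other actor to BP_ThirdPersonCharacter, halve MaxSprintSpeed on entry and set IsOverlapping.
; Exit clears the flag and restores a hard-coded default rather than the previous speed.
; BeginPlay caches the player in PlayerRef, but neither it nor IsOverlapping is read here.
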(event OnComponentBeginOverlap(TriggerBox)
  (params (OverlappedComponent :type Primitive%20Component%20Object%20Reference) (OtherActor :type Actor%20Object%20Reference) (OtherComp :type Primitive%20Component%20Object%20Reference) (OtherBodyIndex :type Integer) (bFromSweep :type Boolean) (SweepResult :type Hit%20Result%20Structure%20%28by%20ref%29))
  (bind _asbp_third_person_character (Utilities|Casting|CastToBP_ThirdPersonCharacter OtherActor))
  (Utilities|IsValid _asbp_third_person_character
    (:Is%20Valid
      (Variables|/Game/Player_Blueprints/BP_ThirdPersonCharacter.BP_ThirdPersonCharacter_C|SetMax_Sprint_Speed _asbp_third_person_character 3e+02)
      (Variables|Default|SetIsOverlapping true))))

(event OnComponentEndOverlap(TriggerBox)
  (params (OverlappedComponent :type Primitive%20Component%20Object%20Reference) (OtherActor :type Actor%20Object%20Reference) (OtherComp :type Primitive%20Component%20Object%20Reference) (OtherBodyIndex :type Integer))
  (bind _asbp_third_person_character (Utilities|Casting|CastToBP_ThirdPersonCharacter OtherActor))
  (Utilities|IsValid _asbp_third_person_character
    (:Is%20Valid
      (Variables|/Game/Player_Blueprints/BP_ThirdPersonCharacter.BP_ThirdPersonCharacter_C|SetMax_Sprint_Speed _asbp_third_person_character 6e+02)
      (Variables|Default|SetIsOverlapping false))))

(event EventBeginPlay
  (bind _asbp_third_person_character (Utilities|Casting|CastToBP_ThirdPersonCharacter (Game|GetPlayerCharacter 0)))
  (Variables|Default|SetPlayer%20Ref _asbp_third_person_character))

(event Collision|EventActorBeginOverlap
  (params (OtherActor :type Actor%20Object%20Reference)))

(event EventTick
  (params (DeltaSeconds :type Float%20%28single-precision%29)))

(fn ConstructionScript)