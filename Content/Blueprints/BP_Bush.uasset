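; BP_Bush is a bush actor that reacts with leaf particles and sound when the third-person character sprints into it.
; Its construction script looks up the Item data table row, sets the bush mesh and stores the row as ItemInfo.
; TriggerZone overlap checks the player's Sprint flag before spawning LeafFX (auto-destroy off) and playing audio.
; Leaving the zone stops the audio after a short delay.
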(event OnComponentBeginOverlap(TriggerZone)
  (params (OverlappedComponent :type Primitive%20Component%20Object%20Reference) (OtherActor :type Actor%20Object%20Reference) (OtherComp :type Primitive%20Component%20Object%20Reference) (OtherBodyIndex :type Integer) (bFromSweep :type Boolean) (SweepResult :type Hit%20Result%20Structure%20%28by%20ref%29))
  (bind _asbp_third_person_character (Utilities|Casting|CastToBP_ThirdPersonCharacter OtherActor))
  (bind _output_get (Variables|Default|SetPlayer%20Ref _asbp_third_person_character))
  (if (Variables|/Game/Player_Blueprints/BP_ThirdPersonCharacter.BP_ThirdPersonCharacter_C|GetSprint? _output_get)
    (Niagara|SpawnSystematLocation (Variables|Default|GetLeafFX) (Transformation|GetWorldLocation (Variables|Default|GetBush)) "0, 0, 0" "1.000000,1.000000,1.000000" false)
    (Audio|Components|Audio|Play (Variables|Default|GetAudio) 0.0)))

(event OnComponentEndOverlap(TriggerZone)
  (params (OverlappedComponent :type Primitive%20Component%20Object%20Reference) (OtherActor :type Actor%20Object%20Reference) (OtherComp :type Primitive%20Component%20Object%20Reference) (OtherBodyIndex :type Integer))
  (bind _asbp_third_person_character (Utilities|Casting|CastToBP_ThirdPersonCharacter OtherActor))
  (Utilities|IsValid _asbp_third_person_character
    (:Is%20Valid
      (Utilities|FlowControl|Delay 0.5)
      (Audio|Components|Audio|Stop (Variables|Default|GetAudio)))))

(event EventBeginPlay)

(event Collision|EventActorBeginOverlap
  (params (OtherActor :type Actor%20Object%20Reference)))

(event EventTick
  (params (DeltaSeconds :type Float%20%28single-precision%29)))

(fn ConstructionScript
  (bind _item (Variables|Default|GetItem))
  (bind _returnvalue (Utilities|GetDataTableRow (.datatable _item) (.rowname _item))
    (:then
      (Components|StaticMesh|SetStaticMesh (Variables|Default|GetBush) (.ItemMesh (Utilities|Struct|BreakS_Bush _returnvalue)))
      (Variables|Default|SetItemInfo _returnvalue))))