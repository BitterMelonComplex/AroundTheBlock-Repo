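; BP_Garlic_Spawner periodically spawns BP_Garlic characters up to a maximum live count.
; If ShouldSpawn is set at BeginPlay, a looping timer fires SpawnGarlic, which spawns at the Sphere's location while below the cap.
; Each new garlic receives a reference to the spawner, launches upward and plays a hop montage.
; OnGarlicDestroyed decrements the live count, freeing a slot for a later timer tick.
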(event Custom|Spawn%20Garlic
  (if (< (Variables|Default|GetCurrent%20Garlic%20Spawned) (Variables|Default|GetMax%20Garlic%20Spawn))
    (Development|PrintString "Spawn")
    ;[1 1 1] Spawn Garlic
    (Math|Integer|IncrementInt (Variables|Default|GetCurrent%20Garlic%20Spawned)
      (:%20%20
        (bind _returnvalue (Game|SpawnActorfromClass "/Game/Characters/NPC/BP_Garlic.BP_Garlic_C" (Math|Transform|MakeTransform (Transformation|GetWorldLocation (Variables|Default|GetSphere)) "0, 0, 0" "1.000000,1.000000,1.000000") "Undefined" "MultiplyWithRoot" 0 0))
        (Variables|/Game/Characters/NPC/BP_Garlic.BP_Garlic_C|SetGarlic%20Spawner _returnvalue self)
        (Character|LaunchCharacter _returnvalue "0.000000,0.000000,200.000000" false false)
        (Animation|PlayAnimMontage _returnvalue "/Game/Characters/Garlic/Garlic_Hop_Montage.Garlic_Hop_Montage" 1.0 "None")))))

(event EventBeginPlay
  (if (Variables|Default|GetShould%20Spawn)
    (Variables|Default|SetShould%20Spawn false)
    (Utilities|Time|SetTimerbyEvent (delegate Custom|Spawn%20Garlic) (Variables|Default|GetSpawn%20Interval) true)))

(event EventOnGarlicDestroyed
  (Math|Integer|DecrementInt (Variables|Default|GetCurrent%20Garlic%20Spawned)
    (:%20%20
      (Development|PrintString "destroyed"))))

(fn ConstructionScript)