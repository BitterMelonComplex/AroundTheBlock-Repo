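; BP_CollectableItem is a world item that is added to the player's inventory when picked up.
; An ItemInfo data table row handle defines the item, and the construction script uses that row to set the static mesh.
; BeginPlay caches the third-person character.
; The ContinueDialogue event checks that the row exists, passes its row name to the character's InventoryComponent, then destroys the actor.
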(event EventBeginPlay
  (bind _asbp_third_person_character (Utilities|Casting|CastToBP_ThirdPersonCharacter (Game|GetPlayerCharacter 0)))
  (Variables|Default|SetPlayerRef _asbp_third_person_character))

(event Collision|EventActorBeginOverlap
  (params (OtherActor :type Actor%20Object%20Reference)))

(event EventTick
  (params (DeltaSeconds :type Float%20%28single-precision%29)))

(event EventContinueDialogue
  (bind _iteminfo (Variables|Default|GetItemInfo))
  (bind _returnvalue (Utilities|GetDataTableRow (.datatable _iteminfo) (.rowname _iteminfo))
    (:then
      (Default|AddtoInventory (Variables|/Game/Player_Blueprints/BP_ThirdPersonCharacter.BP_ThirdPersonCharacter_C|GetInventoryComponent (Variables|Default|GetPlayerRef)) (.rowname _iteminfo))
      (Actor|DestroyActor))))

(fn ConstructionScript
  (bind _iteminfo (Variables|Default|GetItemInfo))
  (bind _returnvalue (Utilities|GetDataTableRow (.datatable _iteminfo) (.rowname _iteminfo))
    (:then
      (Components|StaticMesh|SetStaticMesh (Variables|Default|GetItem) (.InWorldMesh (Utilities|Struct|BreakF_Inventory _returnvalue))))))