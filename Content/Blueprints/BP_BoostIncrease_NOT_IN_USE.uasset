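; Garlic character actor, marked not in use by its name, that animates on player contact and can grant a boost increase.
; Any overlap fires the player's OnGarlicSpawn dispatcher, which it binds to its spawn animation.
; Player overlap also starts a run animation while a timeline lerps the mesh toward a random reachable point within RunAroundIn's radius.
; ContinueDialogue updates the player's boost value and destroys the actor.
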(event OnComponentBeginOverlap(PlayerCollision)
  (params (OverlappedComponent :type Primitive%20Component%20Object%20Reference) (OtherActor :type Actor%20Object%20Reference) (OtherComp :type Primitive%20Component%20Object%20Reference) (OtherBodyIndex :type Integer) (bFromSweep :type Boolean) (SweepResult :type Hit%20Result%20Structure%20%28by%20ref%29))
  (bind _runaroundin (Variables|Default|GetRunAroundIn))
  (bind _playerref (Variables|Default|GetPlayerRef))
  (Default|CallOnGarlicSpawn _playerref)
  (if (== OtherActor _playerref)
    (CallFunction|Spawn)
    (Utilities|FlowControl|Delay 0.4)
    (Components|Animation|PlayAnimation (Variables|Default|GetGarlic%20Boi) "/Game/Characters/Garlic/Garlic_Run.Garlic_Run" true)
    (Variables|Default|SetRandom%20Location (.RandomLocation (AI|Navigation|GetRandomReachablePointinRadius (Transformation|GetWorldLocation _runaroundin) (Components|Sphere|GetScaledSphereRadius _runaroundin) 0 0)))
    (bind _go (Timeline|RunAround PlayFromStart)
      (:Update
        (Transformation|SetWorldLocation (Variables|Default|GetGarlic%20Boi) (Math|Vector|Lerp(Vector) (Transformation|GetWorldLocation (Variables|Default|GetGarlic%20Boi)) (Variables|Default|GetRandom%20Location) _go) false false)))))

(event Custom|Spawn
  (Components|Animation|PlayAnimation (Variables|Default|GetGarlic%20Boi) "/Game/Characters/Garlic/Garlic_Spawn.Garlic_Spawn" false))

(event EventBeginPlay
  (bind _asbp_third_person_character (Utilities|Casting|CastToBP_ThirdPersonCharacter (Game|GetPlayerCharacter 0)))
  (Variables|Default|SetPlayerRef _asbp_third_person_character)
  (Components|Animation|PlayAnimation (Variables|Default|GetGarlic%20Boi) "/Game/Characters/Garlic/Garlic_Idle.Garlic_Idle" true)
  (EventDispatchers|BindEventtoOnGarlicSpawn (Variables|Default|GetPlayerRef) (delegate Custom|Spawn)))

(event EventContinueDialogue
  (Default|UpdateBoostValue (Variables|Default|GetPlayerRef) 1.0)
  (Actor|DestroyActor))

(fn ConstructionScript)