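; BP_Car is a car actor that moves along the spline of a referenced actor, starting at BeginPlay.
; A timeline track is lerped across the spline length to set world location and rotation each update, so the car follows the path's orientation.
; The timeline's play rate is the inverse of TimeToComplete, letting that variable control the travel duration.
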(event Custom|Move%20Object
  (bind _spline (Variables|Default|GetSpline))
  (bind _spline_2 (Variables|/Game/Blueprints/BP_Spline.BP_Spline_C|GetSpline _spline))
  (Components|Timeline|SetPlayRate (Variables|Default|GetT_Move) (/ 1.0 (Variables|Default|GetTime%20to%20complete)))
  (bind _move_track (Timeline|T_Move Play)
    (:Update
      (Transformation|SetActorLocationAndRotation (Spline|GetLocationatDistanceAlongSpline _spline_2 (Math|Float|Lerp 0.0 (Spline|GetSplineLength _spline_2) _move_track) "World") (Spline|GetRotationatDistanceAlongSpline _spline_2 (Math|Float|Lerp 0.0 (Spline|GetSplineLength _spline_2) _move_track) "World")))))

(event EventBeginPlay
  (CallFunction|MoveObject))

(event EventTick
  (params (DeltaSeconds :type Float%20%28single-precision%29)))

(fn ConstructionScript)