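; Bush-like spawner that releases a beetle or a trash bottle when a sprinting third-person character enters its trigger zone.
; Each hit plays leaf FX and sound, while a timed DoOnce gates a random roll that picks a bottle, if under its cap, or otherwise a beetle.
; Capped, cooldown-limited spawns are launched upward, with beetles fleeing shortly after.
; Spawned actors receive a spawner reference, and destroyed events decrement the counts.
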(event OnComponentBeginOverlap(TriggerZone)
  (params (OverlappedComponent :type Primitive%20Component%20Object%20Reference) (OtherActor :type Actor%20Object%20Reference) (OtherComp :type Primitive%20Component%20Object%20Reference) (OtherBodyIndex :type Integer) (bFromSweep :type Boolean) (SweepResult :type Hit%20Result%20Structure%20%28by%20ref%29))
  ;[1 1 1] Spawn leaves when overlap
  (bind _asbp_third_person_character (Utilities|Casting|CastToBP_ThirdPersonCharacter OtherActor))
  (Utilities|IsValid _asbp_third_person_character
    (:Is%20Valid
      (if (Variables|/Game/Player_Blueprints/BP_ThirdPersonCharacter.BP_ThirdPersonCharacter_C|GetSprint? _asbp_third_person_character)
        (Utilities|FlowControl|Sequence
          (:then_0
            (Niagara|SpawnSystematLocation (Variables|Default|GetLeafFX) (Transformation|GetWorldLocation (Variables|Default|GetTrigger%20Zone)) "0, 0, 0" "1.000000,1.000000,1.000000" false)
            (Audio|Components|Audio|Play (Variables|Default|GetBushHit) 0.0)
            (Utilities|FlowControl|Delay 0.5)
            (Audio|Components|Audio|Stop (Variables|Default|GetBushHit))
            (Utilities|FlowControl|Delay 4.0)
            (goto _label Reset))
          (:then_1
            (Utilities|FlowControl|DoOnce false :!label _label
              (:Completed
                ;[1 1 1] Determins if spawner will spawn botle or beetle
                (bind _output_get (Variables|Default|SetCurrentRoll (Math|Random|RandomFloatinRange 0.0 1.0)))
                (if (and (<= _output_get (Variables|Default|Getspawn%20probability)) (< (Variables|Default|GetCurrent%20Bottle%20Spawn) (Variables|Default|GetMax%20Bottle%20Spawn)))
                  ;[1 1 1] Spawn Bottle Logic
                  (if (not (Variables|Default|GetIs%20On%20Cool%20Down))
                    (Variables|Default|SetIs%20On%20Cool%20Down true)
                    (Variables|Default|SetShould%20Spawn true)
                    (if (< (Variables|Default|GetCurrent%20Bottle%20Spawn) (Variables|Default|GetMax%20Bottle%20Spawn))
                      (Audio|Components|Audio|Stop (Variables|Default|GetBugBuzz))
                      (Math|Integer|IncrementInt (Variables|Default|GetCurrent%20Bottle%20Spawn)
                        (:%20%20
                          (bind _returnvalue (Game|SpawnActorfromClass "/Game/Assets/Trash/BP_Bottle.BP_Bottle_C" (Math|Transform|MakeTransform (Transformation|GetWorldLocation (Variables|Default|GetSphere)) "0, 0, 0" "1.000000,1.000000,1.000000") "Undefined" "MultiplyWithRoot" 0 0))
                          (Variables|/Game/Assets/Trash/BP_Bottle.BP_Bottle_C|SetBeetle%20Spawner _returnvalue self)
                          (bind _output_get_2 (Variables|Default|SetXY%20Velocity (Math|Random|RandomFloatinRange -4e+02 4e+02)))
                          (Character|LaunchCharacter _returnvalue (Math|Vector|MakeVector _output_get_2 _output_get_2 5e+02) false false)
                          (Utilities|FlowControl|Delay 6.0)
                          (Variables|Default|SetIs%20On%20Cool%20Down false)
                          (Audio|Components|Audio|Play (Variables|Default|GetBugBuzz) 0.0)))))
                  (else
                    ;[1 1 1] Spawn Beetle based on cool down so only one spawns at a time and on interval
                    (if (not (Variables|Default|GetIs%20On%20Cool%20Down))
                      (Variables|Default|SetIs%20On%20Cool%20Down true)
                      (Variables|Default|SetShould%20Spawn true)
                      (if (< (Variables|Default|GetCurrent%20Beetles%20Spawned) (Variables|Default|GetMax%20Beetles%20Spawn))
                        (Audio|Components|Audio|Stop (Variables|Default|GetBugBuzz))
                        (Development|PrintString "Beetle Spawn")
                        (Math|Integer|IncrementInt (Variables|Default|GetCurrent%20Beetles%20Spawned)
                          (:%20%20
                            (bind _returnvalue_2 (Game|SpawnActorfromClass "/Game/Characters/NPC/BP_Beetle.BP_Beetle_C" (Math|Transform|MakeTransform (Transformation|GetWorldLocation (Variables|Default|GetSphere)) "0, 0, 0" "1.000000,1.000000,1.000000") "Undefined" "MultiplyWithRoot" 0 (Variables|Default|GetBeetle%20Material) 0))
                            ;;[0 0.09584 1] Select Tag from container
                            (GameplayTags|AddGameplayTag :TagContainer (Variables|Default|GetBeetle%20Tags) :!class /Script/GameplayTags.BlueprintGameplayTagLibrary)
                            (Variables|/Game/Characters/NPC/BP_Beetle.BP_Beetle_C|SetBeetle%20Spawner _returnvalue_2 self)
                            (bind _output_get_3 (Variables|Default|SetXY%20Velocity (Math|Random|RandomFloatinRange -4e+02 4e+02)))
                            (Character|LaunchCharacter _returnvalue_2 (Math|Vector|MakeVector _output_get_3 _output_get_3 5e+02) false false)
                            (Animation|PlayAnimMontage _returnvalue_2 "/Game/Characters/Beetle/Beetle_Jump_Montage.Beetle_Jump_Montage" 1.0 "None")
                            (Utilities|FlowControl|Delay 1.0)
                            (Default|Flee _returnvalue_2)
                            (Utilities|FlowControl|Delay 5.0)
                            (Variables|Default|SetIs%20On%20Cool%20Down false)
                            (Audio|Components|Audio|Play (Variables|Default|GetBugBuzz) 0.0)))))))))))))))

(event EventBeginPlay)

(event EventOnBeetleDestroyed
  ;[1 1 1] Beetle Destroyed
  (Math|Integer|DecrementInt (Variables|Default|GetCurrent%20Beetles%20Spawned)
    (:%20%20
      (Development|PrintString "Beetle Destroyed"))))

(event EventOnTrashBottleDestroyed
  ;[1 1 1] Bottle Destroyed
  (Math|Integer|DecrementInt (Variables|Default|GetCurrent%20Bottle%20Spawn)
    (:%20%20
      (Development|PrintString "Bottle Destroyed"))))

(fn ConstructionScript)