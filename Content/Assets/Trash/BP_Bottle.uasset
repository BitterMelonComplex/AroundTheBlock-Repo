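; BP_Bottle is a trash bottle actor, marked with a sparkle effect, that reports its removal to a beetle spawner.
; On BeginPlay it attaches a Niagara sparkle and starts a five-minute self-destruct timer.
; Either that timer or the ContinueDialogue event calls OnTrashBottleDestroyed on the BeetleSpawner, then destroys the actor.
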(event Custom|SelfDestruc
  (Default|OnTrashBottleDestroyed (Variables|Default|GetBeetle%20Spawner))
  (Actor|DestroyActor))

(event EventBeginPlay
  (Utilities|Time|SetTimerbyEvent (delegate Custom|SelfDestruc) 3e+02)
  (Niagara|SpawnSystemAttached "/Game/FX/NS_Sparkle.NS_Sparkle" (Variables|Default|GetSparkle%20FX) "" (Math|Vector|MakeVector 0.0 0.0 0.0) "0, 0, 0" "KeepRelativeOffset" true))

(event EventContinueDialogue
  ;[1 1 1] Destroy Bottle
  (Default|OnTrashBottleDestroyed (Variables|Default|GetBeetle%20Spawner))
  (Actor|DestroyActor))

(fn ConstructionScript)